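; BP_Rupee is a collectible rupee actor that awards a point and can recolor a set of walls.
; The Ber function destroys the actor, increments Point on BP_ThirdPersonGameMode and prints a Point value.
; The custom event ahoj uses a FlipFlop to alternate every Wall entry between red and blue materials across four slots.
; The overlap event is empty, and nothing in this Blueprint calls either Ber or ahoj.
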(event Custom|ahoj
  (Utilities|FlowControl|FlipFlop
    (:A
      (for _array_element (Variables|Default|GetWall)
        (for _index (range 0 3)
          (Rendering|Material|SetMaterial (Variables|/Script/Engine.StaticMeshActor|GetStaticMeshComponent _array_element) _index "/Game/moje/M_Red.M_Red"))))
    (:B
      (for _array_element_2 (Variables|Default|GetWall)
        (for _index_2 (range 0 3)
          (Rendering|Material|SetMaterial (Variables|/Script/Engine.StaticMeshActor|GetStaticMeshComponent _array_element_2) _index_2 "/Game/moje/M_Blue.M_Blue"))))))

(event EventBeginPlay)

(event Collision|EventActorBeginOverlap
  (params (OtherActor :type Actor%20Object%20Reference)))

(event EventTick
  (params (DeltaSeconds :type Float%20%28single-precision%29)))

(fn ConstructionScript)

(fn Ber
  (Actor|DestroyActor)
  (bind _asbp_third_person_game_mode (Utilities|Casting|CastToBP_ThirdPersonGameMode (Game|GetGameMode)))
  (bind _result (Math|Integer|IncrementInt (Variables|/Game/ThirdPerson/Blueprints/BP_ThirdPersonGameMode.BP_ThirdPersonGameMode_C|Getpoint _asbp_third_person_game_mode))
    (:%20%20
      (Development|PrintString (Utilities|String|ToString(Integer) _result)))))