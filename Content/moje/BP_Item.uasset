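; BP_Item is a pickup item actor that adds its LifePoints to a life or heal value supplied by the caller.
; PickupFunction destroys the item and returns the increased value, while PickUpItems returns the sum and leaves the actor in place.
; A separate PickupEvent destroys the item after a short delay.
; It has no active overlap or tick logic, so pickup must be triggered externally.
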(event Custom|PickupEvent
  (Utilities|FlowControl|Delay 0.2)
  (Actor|DestroyActor))

(event EventBeginPlay)

(event Collision|EventActorBeginOverlap
  (params (OtherActor :type Actor%20Object%20Reference)))

(event EventTick
  (params (DeltaSeconds :type Float%20%28single-precision%29)))

(fn ConstructionScript)

(fn PickupFunction
  (params (Life%20In :type Integer))
  (Actor|DestroyActor)
  (return (+ Life%20In (Variables|Default|GetLifePoints))))

(fn PickUpItems
  (params (Heals%20in :type Integer))
  (return (+ Heals%20in (Variables|Default|GetLifePoints))))