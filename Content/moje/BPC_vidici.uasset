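; AI controller that feeds sightings of the player into its Blackboard.
; On perception updates it ignores everything except sight stimuli from player pawn 0.
; It sets targetObject to the player while sensed and clears it when sight is lost.
; Each such update also writes the stimulus location to targetLocation, including the one where sight is lost.
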(event OnTargetPerceptionUpdated(AIPerception)
  (params (Actor :type Actor%20Object%20Reference) (Stimulus :type AI%20Stimulus%20Structure))
  (bind (_age _expirationage _strength _stimuluslocation _receiverlocation _tag _bsuccessfullysensed) (Utilities|Struct|BreakAIStimulus Stimulus))
  (bind _returnvalue (Game|Player|GetPlayerPawn 0))
  (bind _returnvalue_2 (AI|GetBlackboard 0))
  (bind _returnvalue_3 (Class|AIPerceptionSystem|GetSenseClassforStimulus Stimulus))
  (if (== _returnvalue_3 "/Script/AIModule.AISense_Sight")
    (if (== Actor _returnvalue)
      (AI|Components|Blackboard|SetValueasObject _returnvalue_2 (Utilities|Name|MakeLiteralName "targetObject") (Utilities|SelectObject _returnvalue 0 _bsuccessfullysensed))
      (AI|Components|Blackboard|SetValueasVector _returnvalue_2 (Utilities|Name|MakeLiteralName "targetLocation") _stimuluslocation))))

(fn ConstructionScript)